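; Mummy enemy actor that takes damage and shows it as floating damage text.
; On damage, it takes an item from a named pool, places it above itself with the damage value, then lowers health through its Stats.
; BeginPlay caches the player as Target and starts a delay that leads nowhere.
; The chase logic, which drives Capsule velocity toward Target and yaws Body to face it, is disconnected and never runs.
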(event `self.ReceiveBeginPlay`
  (set `self.Target` (`GameplayStatics.GetPlayerCharacter` 0))
  (`KismetSystemLibrary.Delay` 2.0))

(event `self.TakeDamage`
  (params (Damage :type "Float (single-precision)"))
  (bind (_returnvalue_x _returnvalue_y _returnvalue_z) (`KismetMathLibrary.BreakVector` (`self.K2_GetActorLocation`)))
  (bind _returnvalue (`PoolManager.GetNewItem` (`BlueprintMapLibrary.Map_Find` (`PoolSystem.PoolInstances` (`PoolSystem.GetInstance`)) (`self.DamageTextPoolSystemName`))))
  (`self.K2_SetActorLocation` _returnvalue (`KismetMathLibrary.MakeVector` _returnvalue_x _returnvalue_y (+ _returnvalue_z 100.0)) false true)
  (`self.SetFloatValues` _returnvalue (`|MakeArray` Damage))
  (`EnemyStatComponent.DecreaseHealth` (`self.Stats`) Damage))

(fn `UserConstructionScript`)