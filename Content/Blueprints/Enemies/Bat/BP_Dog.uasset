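; BP_Dog is an enemy actor that takes damage but currently does not move.
; On BeginPlay it stores the player character as Target, then runs a two-second delay that leads nowhere.
; Taking damage spawns damage numbers at its location and lowers health through Stats.
; Unconnected chase logic would drive the capsule's physics velocity toward Target and yaw the body to face it, but never runs.
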(event `self.ReceiveBeginPlay`
  (set `self.Target` (`GameplayStatics.GetPlayerCharacter` 0))
  (`KismetSystemLibrary.Delay` 2.0))

(event `self.TakeDamage`
  (params (Damage :type "Float (single-precision)"))
  (`/Game/Blueprints/StaticFunctions/BF_StaticFunctions.SpawnDamageNumbers` (`KismetMathLibrary.FTrunc` Damage) (`self.K2_GetActorLocation`) (`GameplayStatics.GetGameMode`))
  (`EnemyStatComponent.DecreaseHealth` (`self.Stats`) Damage))

(fn `UserConstructionScript`)