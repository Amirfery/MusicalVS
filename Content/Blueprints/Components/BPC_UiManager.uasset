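; BPC_UiManager is a component that manages player UI: the HUD and the game over screen.
; Initialize binds to BPPlayer's XP and Soul Note events through PlayerController, updating the HUD's XP bar ratio and whole-number Soul Notes text.
; CreatePlayerHUD spawns the HUD widget.
; ShowGameOver displays its widget, switches to UI-only input with a cursor, and pauses both game and player.
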(event `self.ReceiveBeginPlay`)

(event `XPAdded`
  (params (XP :type "Float (double-precision)"))
  (bind _bp_player (`/Game/Blueprints/Character/BP_PlayerController.BP Player` (`self.PlayerController`)))
  (`ProgressBar.SetPercent` (`/Game/UI/Widgets/WBP_PlayerHUD.XPBar` (`self.PlayerHUD`)) (/ (`CharacterSystem.XP` _bp_player) (`CharacterSystem.NeededXpToLevelUp` _bp_player))))

(event `SoulNoteAdded`
  (params (SoulNotes :type "Float (double-precision)"))
  (set `TextBlock.Text` (`|FormatText` "Soul Notes: {Amount}" (`KismetMathLibrary.FTrunc` SoulNotes)) (`/Game/UI/Widgets/WBP_PlayerHUD.SoulNoteText` (`self.PlayerHUD`))))

(fn `CreatePlayerHUD`
  (bind _returnvalue (`|CreateWidget` "/Game/UI/Widgets/WBP_PlayerHUD.WBP_PlayerHUD_C"))
  (bind _output_get (set `self.PlayerHUD` _returnvalue))
  (`UserWidget.AddToViewport` _output_get 0))

(fn `Initialize`
  (bind _playercontroller (`self.PlayerController`)
    (:`then`
      (bind _bp_player (`/Game/Blueprints/Character/BP_PlayerController.BP Player` _playercontroller))
      (add `CharacterSystem.OnXPAdded` _bp_player (`|CreateDelegate` :!event `XPAdded`))
      (add `CharacterSystem.OnSoulNoteAdded` _bp_player (`|CreateDelegate` :!event `SoulNoteAdded`)))
    (:`else`)))

(fn `ShowGameOver`
  (bind _returnvalue (`GameplayStatics.GetPlayerController` 0))
  (bind _returnvalue_2 (`|CreateWidget` "/Game/UI/Widgets/WBP_GameOver.WBP_GameOver_C"))
  (`UserWidget.AddToViewport` _returnvalue_2 0)
  (`WidgetBlueprintLibrary.SetInputMode_UIOnlyEx` _returnvalue _returnvalue_2)
  (set `PlayerController.bShowMouseCursor` true _returnvalue)
  (`GameplayStatics.SetGamePaused` true)
  (`CharacterSystem.SetPaused` (`/Game/Blueprints/Character/BP_PlayerController.BP Player` (`self.PlayerController`)) true))