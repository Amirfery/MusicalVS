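; Player character for a level-up-driven action game, taking enemy contact damage through a Health component that drives the health bar and game over.
; Level-ups pause play for an upgrade panel, offering blessings every tenth level when available, and count overlapping level-ups.
; Weapons and blessings spawn from data tables, with owned weapons upgraded instead.
; Also handles gem vacuum, Pumpkin Head freeze, solo input, map rotation and debug keys.
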(event OnComponentHit(CapsuleComponent)
  (params (HitComponent :type Primitive%20Component%20Object%20Reference) (OtherActor :type Actor%20Object%20Reference) (OtherComp :type Primitive%20Component%20Object%20Reference) (NormalImpulse :type Vector :default "0, 0, 0") (Hit :type Hit%20Result%20Structure%20%28by%20ref%29))
  (bind _health (Variables|Default|GetHealth))
  (if (Actor|ActorHasTag OtherActor "Enemy")
    (bind _asenemy (Utilities|Casting|CastToEnemy OtherActor))
    (Class|HealthComponent|DecreaseHealth _health (Variables|/Script/MusicalVS.Enemy|GetDamage _asenemy))
    (if (<= (Class|HealthComponent|GetCurrentHealth _health) 0.0)
      (Default|ShowGameOver (Variables|/Game/Blueprints/Character/BP_PlayerController.BP_PlayerController_C|GetBPC_UiManager (Variables|Default|GetPlayerController))))))

(event Custom|LevelUp
  (bind _returnvalue (Game|GetPlayerController 0))
  (bind _playercontroller (Variables|Default|GetPlayerController))
  (bind _bpc_uimanager (Variables|/Game/Blueprints/Character/BP_PlayerController.BP_PlayerController_C|GetBPC_UiManager _playercontroller))
  (bind _playerhud (Variables|/Game/Blueprints/Components/BPC_UiManager.BPC_UiManager_C|GetPlayerHUD _bpc_uimanager))
  (if (Variables|Default|GetIsLevelUp)
    (Variables|Default|SetLevelUpQueue (+ (Variables|Default|GetLevelUpQueue) 1))
    (else
      (Variables|Default|SetIsLevelUp true)
      (if (|((((Level+1)%10)==0)&&(Level!=0)) (Variables|Default|GetLevel))
        (bind _returnvalue_2 (Class|CharacterSystem|GetBlessingUpgrades))
        (if (Utilities|Array|IsNotEmpty _returnvalue_2)
          (bind _returnvalue_3 (UserInterface|CreateWidget "/Game/UI/Widgets/Upgrade/WBP_UpgradePanel.WBP_UpgradePanel_C" 0 _returnvalue_2 true))
          (Variables|Default|SetUpgradePanel _returnvalue_3)
          (UserInterface|Viewport|AddtoViewport (stale _output_get) 0 :!label _label)
          (Input|SetInputModeUIOnly _returnvalue (stale _returnvalue_5) "DoNotLock" false)
          (Variables|/Script/Engine.PlayerController|SetbShowMouseCursor _returnvalue true)
          (Game|SetGamePaused true)
          (Class|TickSubsystem|StopTimer (Subsystems|GetTickSubsystem))
          (else
            (bind _returnvalue_4 (Class|CharacterSystem|GetUpgrades 3 :!label _label_2))
            (if (Utilities|Array|IsNotEmpty _returnvalue_4)
              (bind _returnvalue_5 (UserInterface|CreateWidget "/Game/UI/Widgets/Upgrade/WBP_UpgradePanel.WBP_UpgradePanel_C" 0 _returnvalue_4))
              (bind _output_get (Variables|Default|SetUpgradePanel _returnvalue_5))
              (goto _label)
              (else
                _))))
        (else
          (goto _label_2)))
      (Variables|/Script/UMG.TextBlock|SetText (Variables|/Game/UI/Widgets/WBP_PlayerHUD.WBP_PlayerHUD_C|GetLevelText _playerhud) (Utilities|Text|FormatText "Level: {Level}" (+ (Variables|Default|GetLevel) 1)))
      (Progress|SetPercent (Variables|/Game/UI/Widgets/WBP_PlayerHUD.WBP_PlayerHUD_C|GetXPBar _playerhud) 0.0))))

(event Custom|ChangeHealth
  (params (Health :type Float%20%28single-precision%29) (MaxHealth :type Float%20%28single-precision%29) (HealthDelta :type Float%20%28single-precision%29))
  (Default|ChangeHealth (stale EventBeginPlay _output_get) Health))

(event Custom|CollectAllGems
  (bind _outactors (Actor|GetAllActorsOfClass "/Game/Blueprints/Attack/BP_Gem.BP_Gem_C"))
  (for _array_element _outactors
    (Class|XpGem|Collect _array_element self)))

(event Custom|FreezeEnemies
  (bind _outactors (Actor|GetAllActorsOfClass "/Game/Blueprints/Enemies/Zombie/BP_PumpkinHead.BP_PumpkinHead_C"))
  (for _array_element _outactors
    (Actor|Tick|SetActorTickEnabled _array_element)))

(event Input|EnhancedActionEvents|EnhancedInputActionIA_Solo
  (params (ActionValue :type Boolean) (ElapsedSeconds :type Float%20%28double-precision%29) (TriggeredSeconds :type Float%20%28double-precision%29) (InputAction :type Input%20Action%20Object%20Reference :default "/Game/Blueprints/Input/IA_Solo.IA_Solo"))
  (:Started
    (Class|CharacterSystem|StartSolo)))

(event EventBeginPlay
  (EventDispatchers|BindEventtoOnLevelUp (delegate Custom|LevelUp))
  (bind _aswbp_health_bar (Utilities|Casting|CastToWBP_HealthBar (UserInterface|GetUserWidgetObject (Variables|Default|GetWidget))))
  (bind _output_get (Variables|UI|SetHealthBar _aswbp_health_bar))
  (EventDispatchers|BindEventtoOnHealthChanged (Variables|Default|GetHealth) (delegate Custom|ChangeHealth))
  (bind _asbp_player_controller (Utilities|Casting|CastToBP_PlayerController (Game|GetPlayerController 0)))
  (Variables|Default|SetPlayerController _asbp_player_controller))

(event Collision|EventActorBeginOverlap
  (params (OtherActor :type Actor%20Object%20Reference))
  (Utilities|IsValid OtherActor
    (:Is%20Valid
      (if (Actor|ActorHasTag OtherActor "Enemy")
        _))))

(event EventTick
  (params (DeltaSeconds :type Float%20%28single-precision%29))
  (Transformation|SetWorldRotation (Variables|Default|GetMap) (Math|Rotator|MakeRotator 0.0 -9e+01 (.yaw (Pawn|GetControlRotation :!class /Script/Engine.Pawn))) false false))

(event EventTakeDamage
  (params (Damage :type Float%20%28single-precision%29))
  (Class|PlayerStatComponent|DecreaseHealth (Variables|Default|GetStats) Damage))

(event Input|KeyboardEvents|R
  (params (Key :type Key%20Structure :default "None"))
  ;[0.15 0.15 0.15 0.5] Test ritual and soul note conversion
  (:Pressed
    (CallFunction|LevelUp)))

(event Input|KeyboardEvents|K
  (params (Key :type Key%20Structure :default "None"))
  ;[0.15 0.15 0.15 0.5] Test ritual and soul note conversion
  (:Pressed
    (Class|CharacterSystem|AddSoulNote 10)))

(fn ConstructionScript)

(fn RemoveUpgradePanel
  (bind _returnvalue (Game|GetPlayerController 0))
  (Widget|RemovefromParent (Variables|Default|GetUpgradePanel))
  (Input|SetInputModeGameOnly _returnvalue false)
  (Variables|/Script/Engine.PlayerController|SetbShowMouseCursor _returnvalue false)
  (Game|SetGamePaused false)
  (Class|CharacterSystem|SetLowpass false)
  (Variables|Default|SetIsLevelUp false)
  (if (>= (Variables|Default|GetLevelUpQueue) 1)
    (Variables|Default|SetLevelUpQueue (- (Variables|Default|GetLevelUpQueue) 1))))

(fn UpWeapon
  (params (Id :type Name))
  (bind _weapons (Variables|Default|GetWeapons))
  (bind (_value _returnvalue) (Utilities|Map|Find _weapons Id))
  (if _returnvalue
    (Class|WeapnSystem|Upgrade _value)
    (elif (< (Utilities|Map|Length _weapons) 10)
      (bind _returnvalue_2 (Utilities|GetDataTableRow "/Game/Data/DT_Weapons.DT_Weapons" Id)
        (:then
          (bind _returnvalue_3 (Game|SpawnActorfromClass (.weaponclass _returnvalue_2) (Math|Transform|MakeTransform "0, 0, 0") "Undefined" "MultiplyWithRoot" 0 0))
          (Class|CharacterSystem|AddWeapon _returnvalue_3))))))

(fn UpBlessing
  (params (Id :type Name))
  (bind _returnvalue (Utilities|GetDataTableRow "/Game/Data/Blessings/DT_Blessings.DT_Blessings" Id)
    (:then
      (bind _returnvalue_2 (Game|SpawnActorfromClass (.blessingclass _returnvalue) (Math|Transform|MakeTransform "0, 0, 0") "Undefined" "MultiplyWithRoot" 0 0))
      (Class|CharacterSystem|AddBlessing _returnvalue_2)
      (Transformation|AttachActorToActor _returnvalue_2 self "None" "KeepRelative" "KeepRelative" "KeepRelative" false))))