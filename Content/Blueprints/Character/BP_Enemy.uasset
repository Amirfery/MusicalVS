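; BP_Enemy is an enemy that constantly homes in on the player character, which it caches on BeginPlay.
; Each Tick overwrites the capsule's physics velocity with a fixed-speed vector toward the player, including the vertical component.
; The skeletal mesh separately yaws to face the player, with an offset for its forward axis.
; The Delay on BeginPlay leads to nothing, so it does not hold back the chase.
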(event `self.ReceiveBeginPlay`
  (set `self.Target` (`GameplayStatics.GetPlayerCharacter` 0))
  (`KismetSystemLibrary.Delay` 2.0))

(event `self.ReceiveTick`
  (params (DeltaSeconds :type "Float (single-precision)"))
  (bind _returnvalue (`self.K2_GetActorLocation`))
  (bind _returnvalue_2 (`self.K2_GetActorLocation` (`self.Target`)))
  (`PrimitiveComponent.SetPhysicsLinearVelocity` (`self.Capsule`) (* (`KismetMathLibrary.Normal` (- _returnvalue_2 _returnvalue)) 300.0) false "None")
  (`SceneComponent.K2_SetWorldRotation` (`self.SkeletalMesh`) (`KismetMathLibrary.MakeRotator` 0.0 0.0 (- (.yaw (`KismetMathLibrary.FindLookAtRotation` _returnvalue _returnvalue_2)) 90.0)) false false))

(fn `UserConstructionScript`)