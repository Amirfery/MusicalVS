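; Player controller that sets up the player's input and HUD and forwards input to BP_Player.
; On BeginPlay it adds the Enhanced Input mapping context, caches the pawn, initializes the HUD through BPCUiManager and binds to TickSubsystem's level timer.
; Move input follows control yaw, while Jump and Interact call straight into the character.
; Look input, the timer callback and timer start are currently unwired or empty.
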(event `self.ReceiveBeginPlay`
  (bind _returnvalue (subsystem `EnhancedInputLocalPlayerSubsystem`))
  (bind _bpc_uimanager (`self.BPC_UiManager`))
  (`/Engine/EditorBlueprintResources/StandardMacros.IsValid` _returnvalue
    (:`Is Valid`
      (`EnhancedInputSubsystemInterface.AddMappingContext` _returnvalue "/Game/Blueprints/Input/IMC_Default.IMC_Default" 0 (struct))
      (bind _asbp_player (cast `/Game/Blueprints/Character/BP_Player` (`GameplayStatics.GetPlayerCharacter` 0)))
      (set `self.BP Player` _asbp_player)
      (`/Game/Blueprints/Components/BPC_UiManager.CreatePlayerHUD` _bpc_uimanager)
      (set `/Game/Blueprints/Components/BPC_UiManager.PlayerController` self _bpc_uimanager)
      (`/Game/Blueprints/Components/BPC_UiManager.Initialize` _bpc_uimanager)
      (add `TickSubsystem.LevelTimerDelegate` (subsystem `TickSubsystem`) (delegate `CustomEvent`)))))

(event `CustomEvent`
  (params (CurrentTime :type Integer)))

(event `EnhancedInput|/Game/Blueprints/Input/IA_Look`
  (params (ActionValue :type "Vector2D Structure") (ElapsedSeconds :type "Float (double-precision)") (TriggeredSeconds :type "Float (double-precision)") (InputAction :type "InputAction Object Reference" :default "/Game/Blueprints/Input/IA_Look.IA_Look")))

(event `EnhancedInput|/Game/Blueprints/Input/IA_Move`
  (params (ActionValue :type "Vector2D Structure") (ElapsedSeconds :type "Float (double-precision)") (TriggeredSeconds :type "Float (double-precision)") (InputAction :type "InputAction Object Reference" :default "/Game/Blueprints/Input/IA_Move.IA_Move"))
  (bind (_returnvalue_roll _returnvalue_pitch _returnvalue_yaw) (`KismetMathLibrary.BreakRotator` (`self.GetControlRotation`)))
  (bind (_returnvalue_roll_2 _returnvalue_pitch_2 _returnvalue_yaw_2) (`KismetMathLibrary.BreakRotator` (`self.GetControlRotation`)))
  (:`Triggered`
    (`Pawn.AddMovementInput` (`self.BP Player`) (`KismetMathLibrary.GetRightVector` (`KismetMathLibrary.MakeRotator` 0.0 0.0 _returnvalue_yaw_2)) ActionValue_X false)
    (`Pawn.AddMovementInput` (`self.BP Player`) (`KismetMathLibrary.GetForwardVector` (`KismetMathLibrary.MakeRotator` 0.0 0.0 _returnvalue_yaw)) ActionValue_Y false)))

(event `EnhancedInput|/Game/Blueprints/Input/IA_Interact`
  (params (ActionValue :type Boolean) (ElapsedSeconds :type "Float (double-precision)") (TriggeredSeconds :type "Float (double-precision)") (InputAction :type "InputAction Object Reference" :default "/Game/Blueprints/Input/IA_Interact.IA_Interact"))
  (:`Triggered`
    (`KismetSystemLibrary.PrintString` "interact pressed")
    (`CharacterSystem.OnInteractPressed` (`self.BP Player`))))

(event `EnhancedInput|/Game/Blueprints/Input/IA_Jump`
  (params (ActionValue :type Boolean) (ElapsedSeconds :type "Float (double-precision)") (TriggeredSeconds :type "Float (double-precision)") (InputAction :type "InputAction Object Reference" :default "/Game/Blueprints/Input/IA_Jump.IA_Jump"))
  (:`Started`
    (`Character.Jump` (`self.BP Player`))))

(fn `UserConstructionScript`)