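; Floating damage number actor that shows a damage value in a WBP_DamageText widget.
; SetFloatValues takes the first float as damage, writes it to the widget text, then calls FreeItem after a half-second delay to release the actor.
; Each Tick moves it upward by a fixed, frame-rate-dependent step and billboards it by copying the camera rotation and flipping yaw.
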(event `self.ReceiveBeginPlay`)

(event `self.ReceiveTick`
  (params (DeltaSeconds :type "Float (single-precision)"))
  (bind (_returnvalue_roll _returnvalue_pitch _returnvalue_yaw) (`KismetMathLibrary.BreakRotator` (`PlayerCameraManager.GetCameraRotation` (`GameplayStatics.GetPlayerCameraManager` 0))))
  (`self.K2_AddActorWorldOffset` (0.0 0.0 5.0))
  (`self.K2_SetActorRotation` (`KismetMathLibrary.MakeRotator` _returnvalue_roll _returnvalue_pitch _returnvalue_yaw))
  (`self.K2_AddActorLocalRotation` (`KismetMathLibrary.MakeRotator` 0.0 0.0 180.0)))

(event `self.SetFloatValues`
  (params (FloatValues :type "Array of Float (single-precision) (by ref)"))
  (bind _output_get (set `self.Damage` (`|GetArrayItem` FloatValues)))
  (bind _aswbp_damage_text (cast `/Game/UI/Widgets/WBP_DamageText` (`WidgetComponent.GetUserWidgetObject` (`self.Widget`))))
  (set `TextBlock.Text` (`KismetTextLibrary.Conv_DoubleToText` _output_get "HalfToEven") (`/Game/UI/Widgets/WBP_DamageText.DamageText` _aswbp_damage_text))
  (`KismetSystemLibrary.Delay` 0.5)
  (`self.FreeItem`))

(fn `UserConstructionScript`)