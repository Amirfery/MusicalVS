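; Blueprint function library for showing floating damage numbers at a world location using the NS_DamageNumbers Niagara system.
; SpawnDamageNumbers rounds the damage, splits it into characters and spawns one system per digit, passing the value through the DamageDigit float variable.
; CalculateDigitLocation offsets each digit around the hit point by its index and DamageNumberSpacing, plus random X/Y jitter rolled separately for every digit.
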(fn `CalculateDigitLocation`
  (params (MainLocation :type "Vector Structure") (CharIndex :type Integer) (DamageLength :type Integer) (HitJitter :type "Vector Structure"))
  (returns (SpawnLocation :type "Vector Structure"))
  (locals (DamageNumberSpacing :type "Float (double-precision)" :default 30.0))
  (return (+ (+ MainLocation (* (- CharIndex (/ DamageLength 2)) (`local.DamageNumberSpacing`))) HitJitter)))

(fn `SpawnDamageNumbers`
  (params (DamageAmount :type Integer) (DamageLocation :type "Vector Structure") (World :type "Object Object Reference"))
  (bind _returnvalue (`KismetStringLibrary.Conv_IntToString` (`KismetMathLibrary.Round` (`KismetMathLibrary.Conv_IntToDouble` DamageAmount))))
  (bind _returnvalue_2 (`KismetStringLibrary.Len` _returnvalue))
  (for _index (range _returnvalue_2)
    (bind _returnvalue_3 (`NiagaraFunctionLibrary.SpawnSystemAtLocation` World "/Game/VFX/NS_DamageNumbers.NS_DamageNumbers" (`self.CalculateDigitLocation` DamageLocation _index _returnvalue_2 (`KismetMathLibrary.MakeVector` (`KismetMathLibrary.RandomFloatInRange` -100.0 100.0) (`KismetMathLibrary.RandomFloatInRange` -100.0 100.0)))))
    (`NiagaraComponent.SetVariableFloat` _returnvalue_3 "DamageDigit" (`KismetStringLibrary.Conv_StringToDouble` (`|GetArrayItem` (`KismetStringLibrary.GetCharacterArrayFromString` _returnvalue) _index)))))